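; Stem tower actor that visualizes the live gain of one PulseScore layer, chosen by LayerId, as a tinted vertical bar.
; BeginPlay applies the Tint to the bar's materials and writes the LayerId to the label.
; Each Tick reads the layer's gain from the score state, scales and offsets the bar so it grows upward from its base, and feeds its Gain material parameter.
; A numeric gain readout follows the bar's top.
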(event EventBeginPlay
  (Rendering|Material|SetVectorParameterValueonMaterials (Variables|Default|GetBar) "Tint" (Variables|Default|GetTint))
  (Rendering|Components|TextRender|SetText (Variables|Default|GetLabel) (|GenerictoText (Variables|Default|GetLayerId))))

(event Collision|EventActorBeginOverlap
  (params (OtherActor :type Actor%20Object%20Reference)))

(event EventTick
  (params (DeltaSeconds :type Float%20%28single-precision%29))
  (bind _returnvalue (Class|PulseScoreStatics|GetScoreState))
  (bind _returnvalue_2 (Math|Float|MakeLiteralFloat 4.3e+02))
  (bind _returnvalue_3 (Math|Float|MakeLiteralFloat 3e+01))
  (bind _layerid (Variables|Default|GetLayerId))
  (bind _bar (Variables|Default|GetBar))
  (bind _value (Variables|Default|GetValue))
  (bind _returnvalue_4 (Class|PulseScoreStatics|GetLayerGain _returnvalue _layerid))
  (bind _returnvalue_5 (* _returnvalue_4 _returnvalue_2))
  (bind _returnvalue_6 (+ _returnvalue_3 _returnvalue_5))
  (Transformation|SetRelativeScale3D _bar (Math|Vector|MakeVector 0.95 0.95 (/ _returnvalue_6 (Math|Float|MakeLiteralFloat 1e+02))))
  (Transformation|SetRelativeLocation _bar (Math|Vector|MakeVector 0.0 0.0 (+ (Math|Float|MakeLiteralFloat 12.0) (/ _returnvalue_6 (Math|Float|MakeLiteralFloat 2.0)))) false false)
  (Rendering|Material|SetScalarParameterValueonMaterials _bar "Gain" _returnvalue_4)
  (Transformation|SetRelativeLocation _value (Math|Vector|MakeVector -7e+01 0.0 (+ (Math|Float|MakeLiteralFloat 46.0) _returnvalue_6)) false false)
  (Rendering|Components|TextRender|SetText _value (|GenerictoText _returnvalue_4)))

(fn ConstructionScript)